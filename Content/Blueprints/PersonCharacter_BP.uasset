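; AI-moved human character that carries a weapon in its hand socket, reacts to sight and turns smoothly to face its current enemy.
; Tick updates the anim Blueprint's walking flag and keeps a gun-hold montage playing.
; Vision collider overlaps feed seen/exit callbacks, while successful moves to a given or random reachable point fire MoveCallback, with a pickup montage for given points.
; Death ragdolls the mesh, then destroys the actor after a delay.
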(event `self.ReceiveBeginPlay`
  (bind _ashuman_2_anim_bp (cast `/Game/Blueprints/Animation/Human2_Anim_BP` (`SkeletalMeshComponent.GetAnimInstance` (`self.Mesh`))))
  (set `self.AnimBP` _ashuman_2_anim_bp))

(event `self.ReceiveTick`
  (params (DeltaSeconds :type "Float (single-precision)"))
  (bind _currentenemy (`self.CurrentEnemy`))
  (`self.Anim Montage Update`)
  (`/Engine/EditorBlueprintResources/StandardMacros.IsValid` _currentenemy
    (:`Is Valid`
      (`self.K2_SetActorRotation` (`KismetMathLibrary.RInterpTo` (`self.K2_GetActorRotation`) (`KismetMathLibrary.FindLookAtRotation` (`self.K2_GetActorLocation`) (`self.K2_GetActorLocation` _currentenemy)) DeltaSeconds 5.0)))))

(event `self.VisionCollider.OnComponentBeginOverlap`
  (params (OverlappedComponent :type "PrimitiveComponent Object Reference") (OtherActor :type "Actor Object Reference") (OtherComp :type "PrimitiveComponent Object Reference") (OtherBodyIndex :type Integer) (bFromSweep :type Boolean) (SweepResult :type "HitResult Structure (by ref)"))
  (`self.SomethingSeenCallback` OtherActor))

(event `self.VisionCollider.OnComponentEndOverlap`
  (params (OverlappedComponent :type "PrimitiveComponent Object Reference") (OtherActor :type "Actor Object Reference") (OtherComp :type "PrimitiveComponent Object Reference") (OtherBodyIndex :type Integer))
  (`self.SomethingSeenExitCallback` OtherActor))

(event `self.MoveToLocation`
  (params (loc :type "Vector Structure (by ref)"))
  (`|AIMoveTo` self loc null 15.0
    (:`OnSuccess`
      (`AnimInstance.Montage_Play` (`self.AnimBP`) "/Game/FBX/Anims/Pickup_AM.Pickup_AM" 1.0 "MontageLength" 0.0 true)
      (`self.MoveCallback` :!label _label))))

(event `self.MoveToRandomLocation`
  (`|AIMoveTo` self (`NavigationSystemV1.K2_GetRandomReachablePointInRadius` (`self.K2_GetActorLocation`) 2000.0 null null) null
    (:`OnSuccess`
      (goto _label))))

(event `self.StopMovement`
  (bind _charactermovement (`self.CharacterMovement`))
  (`/Engine/EditorBlueprintResources/StandardMacros.IsValid` _charactermovement
    (:`Is Valid`
      (`MovementComponent.StopMovementImmediately` _charactermovement))))

(event `self.Death`
  (bind _mesh (`self.Mesh`))
  (`PrimitiveComponent.SetSimulatePhysics` _mesh true)
  (`PrimitiveComponent.SetCollisionEnabled` _mesh "QueryAndPhysics")
  (`KismetSystemLibrary.Delay` 3.0)
  (`self.K2_DestroyActor`))

(fn `Anim Montage Update`
  (bind _animbp (`self.AnimBP`))
  (`/Engine/EditorBlueprintResources/StandardMacros.IsValid` _animbp
    (:`Is Valid`
      (set `/Game/Blueprints/Animation/Human2_Anim_BP.IsWalking` (> (`KismetMathLibrary.VSize` (`MovementComponent.Velocity` (`self.CharacterMovement`))) 25.0) _animbp)
      (if (not (`AnimInstance.Montage_IsPlaying` _animbp "/Game/FBX/Anims/Gun1Hold_AM.Gun1Hold_AM"))
        (`AnimInstance.Montage_Play` _animbp "/Game/FBX/Anims/Gun1Hold_AM.Gun1Hold_AM" 1.0 "MontageLength" 0.0 false)))))

(fn `UserConstructionScript`
  (`SceneComponent.K2_AttachToComponent` (`self.Weapon`) (`self.Mesh`) "Hand1_rSocket" "SnapToTarget" "SnapToTarget" "KeepWorld" true))